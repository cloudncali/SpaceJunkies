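; Beam weapon component that spawns a particle beam and deals point damage.
; Start sets a Firing flag and spawns the beam emitter; Stop only clears the flag.
; Tick runs a visibility trace between fixed coordinates and damages the hit actor every frame without checking Firing.
; Hit direction comes from the PSBeam source point, though Start never stores the spawned emitter there.
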(event EventBeginPlay)

(event EventTick
  (params (DeltaSeconds :type Float%20%28single-precision%29))
  (bind _outhit (Collision|LineTraceByChannel "0, 0, 0" "10000.000000, 0, 0" "TraceTypeQuery1" false 0 "None"))
  (Game|Damage|ApplyPointDamage (.HitActor (Collision|BreakHitResult _outhit)) 1e+02 (.OutSourcePoint (Class|ParticleSystemComponent|GetBeamSourcePoint (Variables|Default|GetPS_Beam))) _outhit))

(fn Start
  (params (bInput :type Boolean))
  (Variables|Default|SetbFiring true)
  (Effects|SpawnEmitterAttached "/Game/SpaceJunkies/Art/ParticleEffects/PS_Beam.PS_Beam" 0 "None"))

(fn Stop
  (Variables|Default|SetbFiring false))