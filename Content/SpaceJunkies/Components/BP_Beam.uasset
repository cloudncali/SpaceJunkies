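; BP_Beam is a beam part Blueprint among the SpaceJunkies components, switched on and off through ActivatePart.
; ActivatePart sets the actor's visibility, collision and ticking together from its Active flag, and the construction script defaults the Active variable to false.
; The event graph holds a visibility line trace feeding a very high point damage hit, but it is disconnected from the empty Tick, so it never runs.
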(event EventTick
  (params (DeltaSeconds :type Float%20%28single-precision%29)))

(fn ConstructionScript
  (Variables|Default|SetbActive false))

(fn ActivatePart
  (params (bActive :type Boolean))
  (Rendering|SetActorHiddenInGame (not bActive))
  (Collision|SetActorEnableCollision bActive)
  (Actor|Tick|SetActorTickEnabled bActive)
  (return))