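; Beam weapon part that damages BP_Ore actors in front of it while active.
; Each tick it line-traces forward from the root against Destructible objects and applies fixed damage to a hit ore, unscaled by delta time.
; ActivatePart toggles visibility, collision, ticking and the active flag together.
; The construction script repeats the same trace-and-damage logic when the flag is set.
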(event EventTick
  (params (DeltaSeconds :type Float%20%28single-precision%29))
  (bind _defaultsceneroot (Variables|Default|GetDefaultSceneRoot))
  (bind _returnvalue (Transformation|GetWorldLocation _defaultsceneroot))
  (if (Variables|Default|GetB_Active)
    (bind _outhit (Collision|LineTraceForObjects _returnvalue (+ _returnvalue (* (Math|Vector|GetForwardVector (Transformation|GetWorldRotation _defaultsceneroot)) 2000)) (Utilities|Array|MakeArray "ObjectTypeQuery6") false 0 "None"))
    (bind _asbp_ore (Utilities|Casting|CastToBP_Ore (.HitActor (Collision|BreakHitResult _outhit))))
    (Default|Damage _asbp_ore 25.0 _outhit)))

(fn ConstructionScript
  (bind _defaultsceneroot (Variables|Default|GetDefaultSceneRoot))
  (bind _returnvalue (Transformation|GetWorldLocation _defaultsceneroot))
  (if (Variables|Default|GetB_Active)
    (bind _outhit (Collision|LineTraceForObjects _returnvalue (+ _returnvalue (* (Math|Vector|GetForwardVector (Transformation|GetWorldRotation _defaultsceneroot)) 2000)) (Utilities|Array|MakeArray "ObjectTypeQuery6") false 0 "None"))
    (bind _asbp_ore (Utilities|Casting|CastToBP_Ore (.HitActor (Collision|BreakHitResult _outhit))))
    (Default|Damage _asbp_ore 25.0 _outhit)))

(fn ActivatePart
  (params (bActive :type Boolean))
  (Rendering|SetActorHiddenInGame (not bActive))
  (Collision|SetActorEnableCollision bActive)
  (Actor|Tick|SetActorTickEnabled bActive)
  (Variables|Default|SetB_Active bActive)
  (return))