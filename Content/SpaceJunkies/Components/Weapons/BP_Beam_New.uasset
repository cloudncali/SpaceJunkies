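; BP_Beam_New is a beam weapon actor that damages ore.
; On BeginPlay, if MBActive is set, it fires a single line trace forward from its root against Destructible objects.
; A hit on a BP_Ore calls that actor's Damage with a fixed amount and the hit result.
; It has no active Tick logic and draws no debug trace.
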(event EventBeginPlay
  (bind _defaultsceneroot (Variables|Default|GetDefaultSceneRoot))
  (bind _returnvalue (Transformation|GetWorldLocation _defaultsceneroot))
  (if (Variables|Default|Getm_bActive)
    (bind _outhit (Collision|LineTraceForObjects _returnvalue (+ _returnvalue (* (Math|Vector|GetForwardVector (Transformation|GetWorldRotation _defaultsceneroot)) 2000)) (Utilities|Array|MakeArray "ObjectTypeQuery6") false 0 "None"))
    (bind _asbp_ore (Utilities|Casting|CastToBP_Ore (.HitActor (Collision|BreakHitResult _outhit))))
    (Default|Damage _asbp_ore 25.0 _outhit)))

(event Collision|EventActorBeginOverlap
  (params (OtherActor :type Actor%20Object%20Reference)))

(event EventTick
  (params (DeltaSeconds :type Float%20%28single-precision%29)))

(fn ConstructionScript)