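; BP_Corvette is a personal ship Blueprint with left and right weapon slots that respond to the primary fire input.
; Each slot's child actor is cast to ShipPart and activated on press or deactivated on release, printing a debug message if a cast fails.
; The right slot is handled only if the left cast succeeds.
; The construction script switches both parts off by default.
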(event EventBeginPlay)

(event Collision|EventActorBeginOverlap
  (params (OtherActor :type Actor%20Object%20Reference)))

(event EventTick
  (params (DeltaSeconds :type Float%20%28single-precision%29)))

(event Input|ActionEvents|InputActionPrimaryFire
  (params (Key :type Key%20Structure))
  (bind _weaponslot_left (Variables|Default|GetWeaponSlot_Left))
  (bind _weaponslot_right (Variables|Default|GetWeaponSlot_Right))
  (bind _childactor (Variables|/Script/Engine.ChildActorComponent|GetChildActor _weaponslot_left))
  (bind _childactor_2 (Variables|/Script/Engine.ChildActorComponent|GetChildActor _weaponslot_right))
  (:Pressed
    (bind _asship_part (Utilities|Casting|CastToShipPart _childactor)
      (:then
        (Class|ShipPart|ActivatePart _asship_part true)
        (bind _asship_part_2 (Utilities|Casting|CastToShipPart _childactor_2)
          (:then
            (Class|ShipPart|ActivatePart _asship_part_2 true))
          (:CastFailed
            (Development|PrintString "Cast Failed" :!label _label))))
      (:CastFailed
        (goto _label))))
  (:Released
    (bind _asship_part_3 (Utilities|Casting|CastToShipPart _childactor)
      (:then
        (Class|ShipPart|ActivatePart _asship_part_3 false)
        (bind _asship_part_4 (Utilities|Casting|CastToShipPart _childactor_2)
          (:then
            (Class|ShipPart|ActivatePart _asship_part_4 false))
          (:CastFailed
            (goto _label))))
      (:CastFailed
        (goto _label)))))

(fn ConstructionScript
  (bind _asship_part (Utilities|Casting|CastToShipPart (Variables|/Script/Engine.ChildActorComponent|GetChildActor (Variables|Default|GetWeaponSlot_Left))))
  (Class|ShipPart|ActivatePart _asship_part false)
  (bind _asship_part_2 (Utilities|Casting|CastToShipPart (Variables|/Script/Engine.ChildActorComponent|GetChildActor (Variables|Default|GetWeaponSlot_Right))))
  (Class|ShipPart|ActivatePart _asship_part_2 false))