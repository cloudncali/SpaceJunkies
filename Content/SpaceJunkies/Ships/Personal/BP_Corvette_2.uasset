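; Player-controllable corvette ship in SpaceJunkies, with left and right weapon slots and speed-reactive engine lights.
; The construction script links both slots' child ShipPart actors to the ship, starts them inactive and puts a dynamic emissive material on the hull.
; PrimaryFire press and release activate and deactivate both weapon parts.
; Tick scales emissive strength with forward speed, updating only while speed is at least the acceleration value.
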(event EventBeginPlay)

(event Collision|EventActorBeginOverlap
  (params (OtherActor :type Actor%20Object%20Reference)))

(event EventTick
  (params (DeltaSeconds :type Float%20%28single-precision%29))
  (bind _f_forwardspeed_current (Variables|Default|GetF_ForwardSpeed_Current))
  (bind _f_acceleration (Variables|Default|GetF_Acceleration))
  (if (>= _f_forwardspeed_current _f_acceleration)
    (Rendering|Material|SetScalarParameterValue (Variables|Default|GetEngineLights) "Emissive_Strength" (+ (* (/ _f_forwardspeed_current _f_acceleration) 1e+02) 1e+02) :!class /Script/Engine.MaterialInstanceDynamic)))

(event Input|ActionEvents|InputActionPrimaryFire
  (params (Key :type Key%20Structure))
  (bind _weaponslot_left (Variables|Default|GetWeaponSlot_Left))
  (bind _weaponslot_right (Variables|Default|GetWeaponSlot_Right))
  (bind _childactor (Variables|/Script/Engine.ChildActorComponent|GetChildActor _weaponslot_left))
  (bind _childactor_2 (Variables|/Script/Engine.ChildActorComponent|GetChildActor _weaponslot_right))
  (:Pressed
    (bind _asship_part (Utilities|Casting|CastToShipPart _childactor)
      (:then
        (Class|ShipPart|ActivatePart _asship_part true)
        (bind _asship_part_2 (Utilities|Casting|CastToShipPart _childactor_2)
          (:then
            (Class|ShipPart|ActivatePart _asship_part_2 true))
          (:CastFailed
            (Development|PrintString "Cast Failed" :!label _label))))
      (:CastFailed
        (goto _label))))
  (:Released
    (bind _asship_part_3 (Utilities|Casting|CastToShipPart _childactor)
      (:then
        (Class|ShipPart|ActivatePart _asship_part_3 false)
        (bind _asship_part_4 (Utilities|Casting|CastToShipPart _childactor_2)
          (:then
            (Class|ShipPart|ActivatePart _asship_part_4 false))
          (:CastFailed
            (goto _label))))
      (:CastFailed
        (goto _label)))))

(fn ConstructionScript
  (bind _asship_part (Utilities|Casting|CastToShipPart (Variables|/Script/Engine.ChildActorComponent|GetChildActor (Variables|Default|GetWeaponSlot_Left))))
  (Class|ShipPart|ActivatePart _asship_part false)
  (Variables|/Script/spacejunkies.ShipPart|SetParentShip _asship_part self)
  (bind _asship_part_2 (Utilities|Casting|CastToShipPart (Variables|/Script/Engine.ChildActorComponent|GetChildActor (Variables|Default|GetWeaponSlot_Right))))
  (Variables|/Script/spacejunkies.ShipPart|SetParentShip _asship_part_2 self)
  (Class|ShipPart|ActivatePart _asship_part_2 false)
  (bind _returnvalue (Rendering|Material|CreateDynamicMaterialInstance "/Game/SpaceJunkies/Art/Ships/M_Corvette01_Emissive_Inst.M_Corvette01_Emissive_Inst" :!class /Script/Engine.KismetMaterialLibrary))
  (bind _output_get (Variables|Default|SetEngineLights _returnvalue))
  (Rendering|Material|SetMaterial (Variables|Default|GetShipMesh) 0 _output_get))