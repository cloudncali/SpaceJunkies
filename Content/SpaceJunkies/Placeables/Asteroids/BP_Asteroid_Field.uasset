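; BP_Asteroid_Field is an asteroid field placeable that spawns a random number of BP_Asteroid actors on BeginPlay.
; The count derives from SpawnMin and SpawnMax, and each position subtracts two random integers per axis within SpawnArea, clustering asteroids around the world origin rather than the field's location.
; Each spawn is followed by a non-uniform SetActorScale3D, randomized per axis between ScaleMin and ScaleMax.
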(event EventBeginPlay
  (bind _spawn_area (Variables|Default|GetSpawn_Area))
  (bind _spawn_area_2 (Variables|Default|GetSpawn_Area))
  (bind _spawn_max (Variables|Default|GetSpawn_Max))
  (bind _spawn_min (Variables|Default|GetSpawn_Min))
  (bind _scale_max (Variables|Default|GetScale_Max))
  (bind _scale_min (Variables|Default|GetScale_Min))
  (bind _returnvalue (- _spawn_max _spawn_min))
  (bind _returnvalue_2 (Math|Random|RandomFloatinRange _scale_min _scale_max))
  (bind (_x _y _z) (Math|Vector|BreakVector _spawn_area))
  (bind (_x_2 _y_2 _z_2) (Math|Vector|BreakVector _spawn_area_2))
  (bind _returnvalue_3 (Math|Random|RandomInteger _returnvalue))
  (bind _returnvalue_4 (+ _returnvalue_3 _spawn_min))
  (Variables|Default|SetSpawn_Total _returnvalue_4)
  (for _index (range 0 _returnvalue_4)
    (bind _output_get (Variables|Default|SetSpawn_Location (Math|Vector|MakeVector (Math|Conversions|ToFloat(Integer) (+ (Math|Random|RandomInteger (Math|Float|Truncate _x)) (* (Math|Random|RandomInteger (Math|Float|Truncate _x_2)) -1))) (Math|Conversions|ToFloat(Integer) (+ (Math|Random|RandomInteger (Math|Float|Truncate _y)) (* (Math|Random|RandomInteger (Math|Float|Truncate _y_2)) -1))) (Math|Conversions|ToFloat(Integer) (+ (Math|Random|RandomInteger (Math|Float|Truncate _z)) (* (Math|Random|RandomInteger (Math|Float|Truncate _z_2)) -1))))))
    (Game|SpawnActorfromClass "/Game/SpaceJunkies/Placeables/Asteroids/BP_Asteroid.BP_Asteroid_C" (Math|Conversions|ToTransform(Vector) _output_get) "Undefined" 0 0)
    (Transformation|SetActorScale3D (Math|Vector|MakeVector _returnvalue_2 _returnvalue_2 _returnvalue_2))))

(event EventTick
  (params (DeltaSeconds :type Float%20%28single-precision%29)))

(event Collision|EventActorBeginOverlap
  (params (OtherActor :type Actor%20Object%20Reference)))

(fn ConstructionScript)