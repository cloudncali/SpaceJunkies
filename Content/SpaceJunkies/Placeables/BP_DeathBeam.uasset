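; BP_DeathBeam is a placeable hazard that fires a damaging beam straight ahead from its root component.
; Every Tick it line-traces 10,000 units along the root's forward vector against two object types, drawing the trace as debug lines.
; A blocking hit applies fixed damage through the hit actor's HealthSystem component, with no validity check and no delta-time scaling, so damage rate follows frame rate.
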(event EventBeginPlay)

(event Collision|EventActorBeginOverlap
  (params (OtherActor :type Actor%20Object%20Reference)))

(event EventTick
  (params (DeltaSeconds :type Float%20%28single-precision%29))
  (bind _defaultsceneroot (Variables|Default|GetDefaultSceneRoot))
  (bind _returnvalue (Transformation|GetWorldLocation _defaultsceneroot))
  (bind _outhit (Collision|LineTraceForObjects _returnvalue (+ _returnvalue (* (Math|Vector|GetForwardVector (Transformation|GetWorldRotation _defaultsceneroot)) 10000)) (Utilities|Array|MakeArray "ObjectTypeQuery7" "ObjectTypeQuery2") false 0 "ForDuration"))
  (if (.bBlockingHit (Collision|BreakHitResult _outhit))
    (Class|HealthSystem|Damage (Actor|GetComponentbyClass (.HitActor (Collision|BreakHitResult _outhit)) "/Script/spacejunkies.HealthSystem") 25.0 _outhit)))

(fn ConstructionScript)