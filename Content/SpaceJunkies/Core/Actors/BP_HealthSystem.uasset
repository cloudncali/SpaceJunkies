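; BP_HealthSystem tracks health for a Space Junkies game object, with temporary immunity after each hit.
; TakeDamage calls Damage, which always stores the last hit info and, unless immune, subtracts health, prints it and starts immunity.
; Tick advances the immunity timer until it reaches its limit, then checks health.
; At zero or below it only sets a Destroy flag, without destroying anything itself.
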(event EventBeginPlay)

(event EventTick
  (params (DeltaSeconds :type Float%20%28single-precision%29))
  (CallFunction|IsImmune DeltaSeconds)
  (CallFunction|IsDead))

(event Custom|TakeDamage
  (params (fDamage :type Float%20%28single-precision%29) (Hit :type Hit%20Result%20Structure))
  (CallFunction|Damage fDamage Hit))

(fn Damage
  (params (fDamage :type Float%20%28single-precision%29) (HitInfo :type Hit%20Result%20Structure))
  (Variables|Default|SetHitInfo_Last HitInfo)
  (if (not (Variables|Default|GetbImmune))
    (bind _output_get (Variables|Default|SetfHealth (- (Variables|Default|GetfHealth) fDamage)))
    (Development|PrintString (Utilities|String|ToString(Float) _output_get))
    (Variables|Default|SetbImmune true)))

(fn IsImmune
  (params (fDeltaTime :type Float%20%28single-precision%29))
  (if (Variables|Default|GetbImmune)
    (bind _output_get (Variables|Default|SetfImmuneTime_Current (+ (Variables|Default|GetfImmuneTime_Current) fDeltaTime)))
    (Math|Float|CompareFloat _output_get (Variables|Default|GetfImmuneTime)
      (:>
        _)
      (:==
        _)
      (:<
        (return true)))
    (bind _output_get_2 (Variables|Default|SetbImmune false))
    (Variables|Default|SetfImmuneTime_Current 0.0)
    (return _output_get_2)
    (else
      (Variables|Default|SetfImmuneTime_Current 0.0)
      (return false))))

(fn IsDead
  (Math|Float|CompareFloat (Variables|Default|GetfHealth) 0.0
    (:>
      (return (Variables|Default|GetbDestroy)))
    (:==
      _)
    (:<
      _))
  (bind _output_get (Variables|Default|SetbDestroy true))
  (return _output_get))