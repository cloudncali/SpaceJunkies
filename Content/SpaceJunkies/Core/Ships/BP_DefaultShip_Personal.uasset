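; BP_DefaultShip_Personal is a ship Blueprint that turns its beam weapons on while the PrimaryFire input is held.
; Press and release events cast the child actors of Weapon1, Weapon2 and Weapon3 to BP_Beam and call ActivatePart with true or false.
; The casts run in series, so a slot that is not a BP_Beam stops the remaining slots from toggling.
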(event EventBeginPlay)

(event Collision|EventActorBeginOverlap
  (params (OtherActor :type Actor%20Object%20Reference)))

(event EventTick
  (params (DeltaSeconds :type Float%20%28single-precision%29)))

(event Input|ActionEvents|InputActionPrimaryFire
  (params (Key :type Key%20Structure))
  (bind _weapon2 (Variables|Default|GetWeapon2))
  (bind _weapon3 (Variables|Default|GetWeapon3))
  (bind _weapon1 (Variables|Default|GetWeapon1))
  (:Pressed
    (bind _asbp_beam (Utilities|Casting|CastToBP_Beam (Variables|/Script/Engine.ChildActorComponent|GetChildActor _weapon1)))
    (Default|ActivatePart _asbp_beam true)
    (bind _asbp_beam_2 (Utilities|Casting|CastToBP_Beam (Variables|/Script/Engine.ChildActorComponent|GetChildActor _weapon2)))
    (Default|ActivatePart _asbp_beam_2 true)
    (bind _asbp_beam_3 (Utilities|Casting|CastToBP_Beam (Variables|/Script/Engine.ChildActorComponent|GetChildActor _weapon3)))
    (Default|ActivatePart _asbp_beam_3 true))
  (:Released
    (bind _asbp_beam_4 (Utilities|Casting|CastToBP_Beam (Variables|/Script/Engine.ChildActorComponent|GetChildActor _weapon1)))
    (Default|ActivatePart _asbp_beam_4 false)
    (bind _asbp_beam_5 (Utilities|Casting|CastToBP_Beam (Variables|/Script/Engine.ChildActorComponent|GetChildActor _weapon2)))
    (Default|ActivatePart _asbp_beam_5 false)
    (bind _asbp_beam_6 (Utilities|Casting|CastToBP_Beam (Variables|/Script/Engine.ChildActorComponent|GetChildActor _weapon3)))
    (Default|ActivatePart _asbp_beam_6 false)))

(fn ConstructionScript)